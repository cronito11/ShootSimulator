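; Target actor that can optionally slide between a start and end location, starting at BeginPlay when Move is set.
; A timeline track drives the position lerp, with play rate set to the inverse of the movement time variable.
; Position updates are skipped while the target is Down, though the timeline keeps running.
; When the timeline finishes, it calls Movement again to continue the motion.
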(event `self.ReceiveBeginPlay`
  (if (`self.Move`)
    (`self.Movement`)))

(event `Movement`
  (`TimelineComponent.SetPlayRate` (`self.Move_TL`) (`KismetMathLibrary.SafeDivide` 1.0 (`self.Miving_Time`)))
  (bind (_direction _newtrack_1) (`Timeline|Move_TL`)
    (:`Update`
      (if (not (`self.Down`))
        (`SceneComponent.K2_SetWorldLocation` (`self.DefaultSceneRoot`) (`KismetMathLibrary.VLerp` (`self.StartLocation`) (`self.EndLocation`) _newtrack_1) false false)))
    (:`Finished`
      (`self.Movement`))))

(fn `UserConstructionScript`)